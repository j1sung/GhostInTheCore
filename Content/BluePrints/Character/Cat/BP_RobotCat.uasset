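; Player-controlled robot cat Character with third-person spring-arm camera and Enhanced Input for looking, camera-relative movement, running and jumping.
; Moving, starting a run and jumping work only in the Locomotion state of StateBP.
; Running uses two timelines to ease walk speed, camera FOV and arm length in and back out when velocity is non-zero.
; BeginPlay sets a downward camera pitch and toggles the collision debug view.
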(event Input|EnhancedActionEvents|EnhancedInputActionIA_View
  (params (ActionValue :type Vector%202D%20Structure) (ElapsedSeconds :type Float%20%28double-precision%29) (TriggeredSeconds :type Float%20%28double-precision%29) (InputAction :type Input%20Action%20Object%20Reference :default "/Game/BluePrints/Input/Actions/IA_View.IA_View"))
  ;[0.15 0.15 0.15 0.5] 회전
  (Pawn|Input|AddControllerYawInput (.x ActionValue)) ; 컨트롤러에 요(Yaw) 회전 추가
  (bind _result (Math|Float|NegateFloat (.y ActionValue)) ; Negate(자연스러움)
    (:%20%20
      (Pawn|Input|AddControllerPitchInput _result) ; 컨트롤러에 피치(Pitch) 회전 추가
    )))

(event Input|EnhancedActionEvents|EnhancedInputActionIA_Jump
  (params (ActionValue :type Boolean) (ElapsedSeconds :type Float%20%28double-precision%29) (TriggeredSeconds :type Float%20%28double-precision%29) (InputAction :type Input%20Action%20Object%20Reference :default "/Game/BluePrints/Input/Actions/IA_Jump.IA_Jump"))
  ;[0.15 0.15 0.15 0.5] 점프
  (:Started
    (switch Utilities|FlowControl|Switch|SwitchonEPlayerState (Variables|Default|GetState_BP)
      (:NewEnumerator0
        (Character|Jump)))))

(event Input|EnhancedActionEvents|EnhancedInputActionIA_Run
  (params (ActionValue :type Boolean) (ElapsedSeconds :type Float%20%28double-precision%29) (TriggeredSeconds :type Float%20%28double-precision%29) (InputAction :type Input%20Action%20Object%20Reference :default "/Game/BluePrints/Input/Actions/IA_Run.IA_Run"))
  ;[0.15 0.04013 0.04874 0.5] 달리기
  (:Started
    (switch Utilities|FlowControl|Switch|SwitchonEPlayerState (Variables|Default|GetState_BP)
      (:NewEnumerator0
        (if (> (Math|Vector|VectorLength (Transformation|GetVelocity self)) 0.0)
          ;;[0.901 0.4349 0.3485 0.5] 달릴때 점점 가속하게 타임라인 사용
          (bind (_direction _walkspeed _fovvalue _targetarmlength) (Timeline|RunTimeline PlayFromStart)
            (:Update
              ;;;[0.15 0.15 0.15 0.5] 이동 속도 가속
              (Variables|/Script/Engine.CharacterMovementComponent|SetMaxWalkSpeed (Variables|Character|GetCharacterMovement) _walkspeed)
              ;;;[0.15 0.15 0.15 0.5] 시야각 넓히기
              (Camera|SetFieldOfView (Variables|Default|GetCamera) _fovvalue)
              ;;;[0.15 0.15 0.15 0.5] 카메라 거리 보정
              (Variables|/Script/Engine.SpringArmComponent|SetTargetArmLength (Variables|Default|GetSpringArm) _targetarmlength)))))))
  (:Completed
    (if (> (Math|Vector|VectorLength (Transformation|GetVelocity self)) 0.0)
      ;;[0.7786 0.6087 0.1618 0.5] 멈출때는 천천히 돌아오게 타임라인 적용
      (bind (_direction_2 _walkspeed_2 _fovvalue_2 _targetarmlength_2) (Timeline|RunTimeline2 PlayFromStart)
        (:Update
          ;;;[0.15 0.15 0.15 0.5] 이동 속도 감속
          (Variables|/Script/Engine.CharacterMovementComponent|SetMaxWalkSpeed (Variables|Character|GetCharacterMovement) _walkspeed_2)
          ;;;[0.15 0.15 0.15 0.5] 시야각 되돌리기
          (Camera|SetFieldOfView (Variables|Default|GetCamera) _fovvalue_2)
          ;;;[0.15 0.15 0.15 0.5] 카메라 거리 되돌리기
          (Variables|/Script/Engine.SpringArmComponent|SetTargetArmLength (Variables|Default|GetSpringArm) _targetarmlength_2))))))

(event Input|EnhancedActionEvents|EnhancedInputActionIA_Move
  (params (ActionValue :type Vector%202D%20Structure) (ElapsedSeconds :type Float%20%28double-precision%29) (TriggeredSeconds :type Float%20%28double-precision%29) (InputAction :type Input%20Action%20Object%20Reference :default "/Game/BluePrints/Input/Actions/IA_Move.IA_Move"))
  ;[0.15 0.15 0.15 0.5] 이동
  (switch Utilities|FlowControl|Switch|SwitchonEPlayerState (Variables|Default|GetState_BP)
    (:NewEnumerator0
      (Pawn|Input|AddMovementInput (Math|Vector|GetRightVector (Pawn|GetControlRotation :!class /Script/Engine.Pawn)) (.x ActionValue) false)
      (Pawn|Input|AddMovementInput (Math|Vector|GetForwardVector (Math|Rotator|MakeRotator 0.0 0.0 (.yaw (Pawn|GetControlRotation :!class /Script/Engine.Pawn)))) (.y ActionValue) false))))

(event EventBeginPlay
  ;[0.15 0.15 0.15 0.5] 카메라 초기 각도 설정
  (Pawn|SetControlRotation (Game|GetPlayerController 0) (Math|Rotator|MakeRotator 0.0 -3e+01 0.0))
  (Development|ExecuteConsoleCommand "Show COLLISION" 0) ; 콜리젼 디버깅
)

(fn ConstructionScript)