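; Player character Blueprint for the robot cat, handling sprinting and the attack input.
; Run start and completion overrides forward to events that play separate timelines, ramping walk speed, camera FOV and spring arm length up and back down.
; Attack input in the Locomotion state switches to Battle and plays the attack montage, while BeginPlay starts with weapon equipping disabled.
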(event Custom|EventApplyRunCompleted
  ;[0.15 0.15 0.15 0.5] 달리기 오버라이딩
  ;;[0.7786 0.6087 0.1618 0.5] 멈출때는 천천히 돌아오게 타임라인 적용
  (bind (_direction _walkspeed _fovvalue _targetarmlength) (Timeline|RunTimeline2 PlayFromStart)
    (:Update
      ;;;[0.15 0.15 0.15 0.5] 이동 속도 감속
      (Variables|/Script/Engine.CharacterMovementComponent|SetMaxWalkSpeed (Variables|Character|GetCharacterMovement) _walkspeed)
      ;;;[0.15 0.15 0.15 0.5] 시야각 되돌리기
      (Camera|SetFieldOfView (Variables|Default|GetCamera) _fovvalue)
      ;;;[0.15 0.15 0.15 0.5] 카메라 거리 되돌리기
      (Variables|/Script/Engine.SpringArmComponent|SetTargetArmLength (Variables|Default|GetSpringArm) _targetarmlength))))

(event Custom|EventApplyRunStarted
  ;[0.15 0.15 0.15 0.5] 달리기 오버라이딩
  ;;[0.901 0.4349 0.3485 0.5] 달릴때 점점 가속하게 타임라인 사용
  (bind (_direction _walkspeed _fovvalue _targetarmlength) (Timeline|RunTimeline PlayFromStart)
    (:Update
      ;;;[0.15 0.15 0.15 0.5] 이동 속도 가속
      (Variables|/Script/Engine.CharacterMovementComponent|SetMaxWalkSpeed (Variables|Character|GetCharacterMovement) _walkspeed)
      ;;;[0.15 0.15 0.15 0.5] 시야각 넓히기
      (Camera|SetFieldOfView (Variables|Default|GetCamera) _fovvalue)
      ;;;[0.15 0.15 0.15 0.5] 카메라 거리 보정
      (Variables|/Script/Engine.SpringArmComponent|SetTargetArmLength (Variables|Default|GetSpringArm) _targetarmlength))))

(event EventBeginPlay
  (|CallParentFunction)
  ;[0.7979 0.4009 0.8333 0.5] 무기 습득 여부 X
  (Variables|Default|SetCanEquipWeapon false))

(event Collision|EventActorBeginOverlap
  (params (OtherActor :type Actor%20Object%20Reference))
  (|CallParentFunction OtherActor) ; This node is disabled and will not be called.\nDrag off pins to build functionality.
)

(event EventTick
  (params (DeltaSeconds :type Float%20%28single-precision%29))
  (|CallParentFunction DeltaSeconds) ; This node is disabled and will not be called.\nDrag off pins to build functionality.
)

(fn ConstructionScript
  (|CallParentFunction))

(fn ApplyRunStarted
  (CallFunction|EventApplyRunStarted))

(fn ApplyRunCompleted
  (CallFunction|EventApplyRunCompleted))

(fn OnIAAttack
  ;[0.15 0.15 0.15 0.5] 일반 상태인지 확인
  (switch Utilities|FlowControl|Switch|SwitchonEPlayerState (Variables|Default|GetState_BP)
    (:NewEnumerator0
      (Variables|Default|SetState_BP "NewEnumerator1")
      (Animation|PlayAnimMontage "/Game/BluePrints/Character/Cat/AM_RobotCat.AM_RobotCat" 1.0 "None"))))