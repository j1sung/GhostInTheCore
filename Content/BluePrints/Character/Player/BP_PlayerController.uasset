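; Player controller that sets up game input and forwards player actions to the controlled BP_BaseCharacter.
; Enhanced Input view, move, run and jump events cast the pawn and call its matching handlers.
; BeginPlay restores game-only input with a hidden cursor, adds IMC_Game and pitches the starting camera down.
; Each tick it projects the current interaction target's offset world position to screen to place the interaction widget.
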(event Input|EnhancedActionEvents|EnhancedInputActionIA_View
  (params (ActionValue :type Vector%202D%20Structure) (ElapsedSeconds :type Float%20%28double-precision%29) (TriggeredSeconds :type Float%20%28double-precision%29) (InputAction :type Input%20Action%20Object%20Reference :default "/Game/BluePrints/Input/Actions/IA_View.IA_View"))
  ;[0.15 0.15 0.15 0.5] 회전
  (bind _asbp_base_character (Utilities|Casting|CastToBP_BaseCharacter (Pawn|GetControlledPawn)))
  (Default|OnIAView _asbp_base_character ActionValue))

(event Input|EnhancedActionEvents|EnhancedInputActionIA_Jump
  (params (ActionValue :type Boolean) (ElapsedSeconds :type Float%20%28double-precision%29) (TriggeredSeconds :type Float%20%28double-precision%29) (InputAction :type Input%20Action%20Object%20Reference :default "/Game/BluePrints/Input/Actions/IA_Jump.IA_Jump"))
  ;[0.15 0.15 0.15 0.5] 점프
  (:Started
    (bind _asbp_base_character (Utilities|Casting|CastToBP_BaseCharacter (Pawn|GetControlledPawn)))
    (Default|OnIAJump _asbp_base_character)))

(event Input|EnhancedActionEvents|EnhancedInputActionIA_Run
  (params (ActionValue :type Boolean) (ElapsedSeconds :type Float%20%28double-precision%29) (TriggeredSeconds :type Float%20%28double-precision%29) (InputAction :type Input%20Action%20Object%20Reference :default "/Game/BluePrints/Input/Actions/IA_Run.IA_Run"))
  ;[0.15 0.15 0.15 0.5] 달리기
  (:Started
    (bind _asbp_base_character (Utilities|Casting|CastToBP_BaseCharacter (Pawn|GetControlledPawn)))
    (Default|OnIARunStarted _asbp_base_character))
  (:Completed
    (bind _asbp_base_character_2 (Utilities|Casting|CastToBP_BaseCharacter (Pawn|GetControlledPawn)))
    (Default|OnIARunCompleted _asbp_base_character_2)))

(event Input|EnhancedActionEvents|EnhancedInputActionIA_Move
  (params (ActionValue :type Vector%202D%20Structure) (ElapsedSeconds :type Float%20%28double-precision%29) (TriggeredSeconds :type Float%20%28double-precision%29) (InputAction :type Input%20Action%20Object%20Reference :default "/Game/BluePrints/Input/Actions/IA_Move.IA_Move"))
  ;[0.15 0.15 0.15 0.5] 이동
  (bind _asbp_base_character (Utilities|Casting|CastToBP_BaseCharacter (Pawn|GetControlledPawn)))
  (Default|OnIAMove _asbp_base_character ActionValue))

(event EventBeginPlay
  ;[0.9297 0.04358 0.1409 0.5] 게임 기본 설정
  ;;[0.15 0.15 0.15 0.5] 게임 재시작(컨트롤러 재설정 시) 마우스 Off
  (Input|SetInputModeGameOnly self false)
  (Variables|Default|SetbShowMouseCursor false)
  (Input|AddMappingContext (PlayerController|LocalPlayerSubsystems|GetEnhancedInputLocalPlayerSubsystem) "/Game/BluePrints/Input/IMC_Game.IMC_Game" 0 "(bIgnoreAllPressedKeysUntilRelease=True,bForceImmediately=False,bNotifyUserSettings=False)")
  (Pawn|SetControlRotation (Math|Rotator|MakeRotator 0.0 -3e+01 0.0)) ; 카메라 처음 회전 각도 보정
)

(event EventTick
  (params (DeltaSeconds :type Float%20%28single-precision%29))
  ;[0.8411 0.3279 0.4373 0.5] 상호작용 처리
  ;;[0.15 0.15 0.15 0.5] 상호작용 액터&위젯 유효성 검사
  (Utilities|IsValid (Variables|Default|GetInteractionUI)
    (:Is%20Valid
      (Utilities|IsValid (Variables|Default|GetCurrentInteractTarget)
        (:Is%20Valid
          (Class|UserWidget|SetPositioninViewport (Variables|Default|GetInteractionUI) (.ScreenPosition (Class|GameplayStatics|ProjectWorldtoScreen self (+ (Transformation|GetActorLocation (Variables|Default|GetCurrentInteractTarget)) (Variables|Default|GetAddUIPos)) false)) true))))))

(fn ConstructionScript)