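; BP_HPController is a component managing shield and HP, with groggy and death states.
; Damage drains the shield first, raising a groggy event when it empties; later hits each remove one HP regardless of damage amount, raising a die event at zero.
; Event dispatchers report shield and HP changes, though the lethal hit fires only the die event.
; Values start at maximum, and UpdateMaxShield resets the shield to a new maximum.
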(event Custom|ReceiveDamage
  (params (Damage :type Float%20%28double-precision%29))
  ;[0.7708 0.2788 0.3267 0.5] 데미지 처리 - 과정에서 죽음 이벤트도 발행
  (if (> (Variables|Default|GetShieldPower) 0.0)
    (bind _output_get (Variables|Default|SetShieldPower (- (Variables|Default|GetShieldPower) Damage)))
    (if (<= _output_get 0.0)
      (Variables|Default|SetShieldPower 0.0)
      (Default|CallOnGroggyEvent)
      ;;[0.15 0.15 0.15 0.5] 쉴드 UI 반영 수치 넘기기
      (Default|CallOnShieldChanged (Variables|Default|GetShieldPower) (Variables|Default|GetMaxShieldPower))
      (else
        ;;[0.15 0.15 0.15 0.5] 쉴드 UI 반영 수치 넘기기
        (Default|CallOnShieldChanged (Variables|Default|GetShieldPower) (Variables|Default|GetMaxShieldPower))))
    (else
      ;;[0.15 0.15 0.15 0.5] 실드가 0인 그로기 상태에 공격받음
      (bind _result (Math|Integer|DecrementInt (Variables|Default|GetHp))
        (:%20%20
          (bind _output_get_2 (Variables|Default|SetHp _result))
          (if (<= _output_get_2 0)
            (Variables|Default|SetHp 0)
            ;;;[0.15 0.15 0.15 0.5] HP횟수 3번 맞으면 죽음 이벤트
            (Default|CallOnDieEvent)
            (else
              (Default|CallOnHPChanged (Variables|Default|GetHp) (Variables|Default|GetMaxHp)))))))))

(event Custom|UpdateMaxShield
  (params (MaxHealthPower :type Float%20%28double-precision%29))
  ;[0.15 0.15 0.15 0.5] 따로 구조체 레벨디자인 하면 사용
  (bind _output_get (Variables|Default|SetMaxShieldPower MaxHealthPower))
  (Variables|Default|SetShieldPower _output_get))

(event EventBeginPlay
  ;[0.8906 0.6686 0.08674 0.5] 시작할 때 최대 수치 초기화
  (Variables|Default|SetShieldPower (Variables|Default|GetMaxShieldPower))
  (Variables|Default|SetHp (Variables|Default|GetMaxHp)))